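; BP_OnlyEnemy is an enemy with helper functions for player detection, wandering, chasing and damage, none called by its empty event graph.
; FindPlayer checks distance and angle, though the angle uses the player's raw world position rather than a normalized direction.
; RandomMove alternates walking and pausing on delta-time timers with periodic random yaw.
; ChasingPlayer faces and steps toward the player by a fixed, frame-dependent offset; OnDamaged only subtracts Hp.
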(event `self.ReceiveTick`
  (params (DeltaSeconds :type "Float (single-precision)")))

(fn `ChasingPlayer`
  (bind _returnvalue (`self.K2_GetActorLocation`))
  (bind _returnvalue_2 (`self.K2_GetActorLocation` (`GameplayStatics.GetPlayerCharacter` 0)))
  (`self.K2_SetActorRotation` (`KismetMathLibrary.FindLookAtRotation` _returnvalue _returnvalue_2))
  (`self.K2_SetActorLocation` (+ _returnvalue (* (`KismetMathLibrary.Normal` (- _returnvalue_2 _returnvalue)) 10.0))))

(fn `FindPlayer`
  (params (dist :type "Float (double-precision)") (angle :type "Float (double-precision)"))
  (returns (isFindPlayer :type Boolean))
  (bind _dist (`self.GetDistance`))
  (bind _angle (`self.GetAngle`))
  (return (and (<= _dist dist) (<= _angle angle))))

(fn `GetAngle`
  (returns (angle :type "Float (double-precision)"))
  (return (`KismetMathLibrary.RadiansToDegrees` (`KismetMathLibrary.Acos` (`KismetMathLibrary.Dot_VectorVector` (`self.K2_GetActorLocation` (`GameplayStatics.GetPlayerCharacter` 0)) (`self.GetActorForwardVector`))))))

(fn `GetDistance`
  (returns (dist :type "Float (double-precision)"))
  (return (`KismetMathLibrary.Vector_Distance` (`self.K2_GetActorLocation` (`GameplayStatics.GetPlayerCharacter` 0)) (`self.K2_GetActorLocation`))))

(fn `OnDamaged`
  (params (Damage :type "Float (double-precision)"))
  (set `self.Hp` (- (`self.Hp`) Damage)))

(fn `RandomMove`
  (returns (isRun :type Boolean))
  (locals (currtime :type "Float (double-precision)"))
  (`self.RandomRotation`)
  (`self.AddMovementInput` (* (`self.GetActorForwardVector`) (`self.forwardInt`)))
  (set `self.currRandTime` (+ (`self.currRandTime`) (`GameplayStatics.GetWorldDeltaSeconds`)))
  (if (> (`self.currRandTime`) 5.0)
    (set `self.forwardInt` 1)
    (set `self.currRandTime` 0.0)
    (return true)
    (elif (> (`self.currRandTime`) 3.0)
      (set `self.forwardInt` 0)
      (return false))))

(fn `RandomRotation`
  (bind _output_get (set `self.currTime` (+ (`self.currTime`) (`GameplayStatics.GetWorldDeltaSeconds`))))
  (if (>= _output_get 5.0)
    (`self.K2_SetActorRotation` (`KismetMathLibrary.MakeRotator` 0.0 0.0 (`KismetMathLibrary.RandomFloatInRange` 0.0 359.0)))
    (set `self.currTime` 0.0)))

(fn `UserConstructionScript`)
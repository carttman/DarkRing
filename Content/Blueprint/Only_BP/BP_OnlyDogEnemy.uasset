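; Dog enemy character that wanders, chases the player and bites at close range, driven by state flags on ABP_OnlyDogEnemy.
; Tick uses FindPlayer to choose between ChasingPlayer and RandomMove, setting the attack flag when within range.
; While attacking, a delay timer ends in a debug-drawn forward sphere trace that damages BP_Player and clears the flag.
; The damaged flag halts this logic, but the damage-reaction chain that sets it here is unconnected.
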(event `self.ReceiveBeginPlay`
  (`parent.ReceiveBeginPlay`)
  (bind _asabp_only_dog_enemy (cast `/Game/Blueprint/Only_BP/ABP_OnlyDogEnemy` (`SkeletalMeshComponent.GetAnimInstance` (`self.Mesh`))))
  (set `self.anim` _asabp_only_dog_enemy))

(event `self.ReceiveTick`
  (params (DeltaSeconds :type "Float (single-precision)"))
  (bind _returnvalue (`self.K2_GetActorLocation`))
  (if (`/Game/Blueprint/Only_BP/ABP_OnlyDogEnemy.isDamaged` (`self.anim`))
    _
    (elif (`/Game/Blueprint/Only_BP/ABP_OnlyDogEnemy.isAttack` (`self.anim`))
      (bind _output_get (set `self.AttackDelayTime` (+ (`self.AttackDelayTime`) DeltaSeconds)))
      (if (> _output_get 3.0)
        (bind _outhit (`KismetSystemLibrary.SphereTraceSingle` :`Start` _returnvalue :`End` (+ _returnvalue (* (`self.GetActorForwardVector`) 80.0)) :`Radius` 50.0 :`TraceChannel` "TraceTypeQuery3" :`DrawDebugType` "ForOneFrame"))
        (bind _asbp_player (cast `/Game/Blueprint/BP_Player` (`.HitActor` (`GameplayStatics.BreakHitResult` _outhit)))
          (:`then`
            (`/Game/Blueprint/BP_Player.TakeDamage` _asbp_player (make `/Game/KEJ/DamageSystem/S_DamageInfo` 5.0 "NewEnumerator1")))
          (:`CastFailed`
            _))
        (set `/Game/Blueprint/Only_BP/ABP_OnlyDogEnemy.isAttack` false (`self.anim`))
        (set `self.AttackDelayTime` 0.0))
      (else
        (bind _isfindplayer (`self.FindPlayer` 5000.0 180.0))
        (if _isfindplayer
          (`self.ChasingPlayer` 10.0)
          (set `/Game/Blueprint/Only_BP/ABP_OnlyDogEnemy.isWalk` false (`self.anim`))
          (set `/Game/Blueprint/Only_BP/ABP_OnlyDogEnemy.isChasing` true (`self.anim`))
          (bind _dist (`self.GetDistance`))
          (if (<= _dist 100.0)
            (set `/Game/Blueprint/Only_BP/ABP_OnlyDogEnemy.isAttack` true (`self.anim`)))
          (else
            (set `/Game/Blueprint/Only_BP/ABP_OnlyDogEnemy.isWalk` true (`self.anim`))
            (set `/Game/Blueprint/Only_BP/ABP_OnlyDogEnemy.isChasing` false (`self.anim`))
            (bind _isrun (`self.RandomMove`))
            (set `/Game/Blueprint/Only_BP/ABP_OnlyDogEnemy.isWalk` _isrun (`self.anim`))))))))

(fn `UserConstructionScript`
  (`parent.UserConstructionScript`))
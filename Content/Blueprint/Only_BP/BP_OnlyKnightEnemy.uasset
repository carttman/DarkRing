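; BP_OnlyKnightEnemy is a melee knight enemy that wanders, spots and chases the player, attacks up close, and dies.
; Tick runs the behavior as a state machine stored in ABP_OnlyKnightEnemy flags, using inherited or external helpers for movement and detection.
; Attacks use a delayed forward sphere trace to damage BP_Player, disengaging when a miss finds the player out of range.
; At zero HP it sets the death flag, then destroys itself after a delay.
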(event `self.ReceiveBeginPlay`
  (`parent.ReceiveBeginPlay`)
  (bind _asabp_only_knight_enemy (cast `/Game/Blueprint/Only_BP/ABP_OnlyKnightEnemy` (`SkeletalMeshComponent.GetAnimInstance` (`self.Mesh`))))
  (set `self.anim` _asabp_only_knight_enemy))

(event `self.ReceiveTick`
  (params (DeltaSeconds :type "Float (single-precision)"))
  (bind _anim (`self.anim`))
  (bind _returnvalue (+ (`self.K2_GetActorLocation`) (10.0 0.0 10.0)))
  (if (<= (`self.Hp`) 0.0)
    (set `/Game/Blueprint/Only_BP/ABP_OnlyKnightEnemy.isAttach` false _anim)
    (set `/Game/Blueprint/Only_BP/ABP_OnlyKnightEnemy.isWalking` false _anim)
    (set `/Game/Blueprint/Only_BP/ABP_OnlyKnightEnemy.isDeath` true _anim)
    (set `/Game/Blueprint/Only_BP/ABP_OnlyKnightEnemy.FindPlayer` false _anim)
    (`KismetSystemLibrary.Delay` 2.0)
    (`self.K2_DestroyActor`)
    (elif (`/Game/Blueprint/Only_BP/ABP_OnlyKnightEnemy.isAttach` (`self.anim`))
      (`KismetSystemLibrary.Delay` 1.5)
      (bind _outhit (`KismetSystemLibrary.SphereTraceSingle` _returnvalue (+ _returnvalue (* (`self.GetActorForwardVector`) 120.0)) 60.0 "TraceTypeQuery3"))
      (bind _asbp_player (cast `/Game/Blueprint/BP_Player` (`.HitActor` (`GameplayStatics.BreakHitResult` _outhit)))
        (:`then`
          (`/Game/KEJ/DamageSystem/BPI_Damagable.TakeDamage` _asbp_player (make `/Game/KEJ/DamageSystem/S_DamageInfo` 10.0 "NewEnumerator1")))
        (:`CastFailed`
          (bind _dist (`self.GetDistance`))
          (if (> _dist 150.0)
            (set `/Game/Blueprint/Only_BP/ABP_OnlyKnightEnemy.isAttach` false (`self.anim`)))))
      (elif (`/Game/Blueprint/Only_BP/ABP_OnlyKnightEnemy.FindPlayer` (`self.anim`))
        (`self.ChasingPlayer` 10.0)
        (bind _dist_2 (`self.GetDistance`))
        (if (< _dist_2 150.0)
          (set `/Game/Blueprint/Only_BP/ABP_OnlyKnightEnemy.isAttach` true (`self.anim`)))
        (else
          (bind _isfindplayer (`self.FindPlayer` 1000.0 30.0))
          (if _isfindplayer
            (set `/Game/Blueprint/Only_BP/ABP_OnlyKnightEnemy.isWalking` false (`self.anim`))
            (set `/Game/Blueprint/Only_BP/ABP_OnlyKnightEnemy.FindPlayer` true (`self.anim`))
            (else
              (bind _isrun (`self.RandomMove`))
              (set `/Game/Blueprint/Only_BP/ABP_OnlyKnightEnemy.isWalking` _isrun (`self.anim`)))))))))

(fn `UserConstructionScript`
  (`parent.UserConstructionScript`))
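; Player actor with health, death and a melee attack that can hit the Darksoul boss.
; BPCDamageSystem handles damage and health, feeds the damage interface functions, and has death and response events bound in the construction script; a widget displays health.
; Left click opens a one-second window where Tick sphere-traces for pawns, damages the first hit and plays a random hit-reaction montage section on the boss.
; Death ragdolls the mesh, disables input and destroys the actor after a delay.
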(event `Death`
  (bind _mesh (`self.Mesh`))
  ;[1 1 1] 사망처리
  (`PrimitiveComponent.SetSimulatePhysics` _mesh true)
  (`PrimitiveComponent.SetCollisionEnabled` _mesh "QueryAndPhysics")
  (`self.DisableInput` (`GameplayStatics.GetPlayerController` 0))
  (`KismetSystemLibrary.Delay` 3.0)
  (`self.K2_DestroyActor`))

(event `self.ReceiveBeginPlay`
  ;[1 1 1] 시작하면 HP바 띄우도록
  (bind _returnvalue (`|CreateWidget` "/Game/KEJ/DamageSystem/W_Health.W_Health_C" null self))
  (`WidgetComponent.SetWidget` (`self.Widget`) _returnvalue))

(event `DamageResponse`
  (params (`Damage Response` :type "/Game/KEJ/DamageSystem/E_DamageResponses Enum" :default "NewEnumerator0"))
  ;[1 1 1] 사망처리
  (`KismetSystemLibrary.PrintString` (`|GetEnumeratorNameAsString` `Damage Response`)))

(event `Key|LeftMouseButton`
  (params (Key :type "Key Structure"))
  ;[1 1 1] 눌른거 체크하면 밑에 스피어 트레이스 발동 되도록
  (:`Pressed`
    (set `self.leftBtnPressed` true)
    (`KismetSystemLibrary.Delay` 1.0)
    (set `self.leftBtnPressed` false)))

(event `self.ReceiveTick`
  (params (DeltaSeconds :type "Float (single-precision)"))
  (if (`self.leftBtnPressed`)
    (bind (_outhit _returnvalue) (`KismetSystemLibrary.SphereTraceSingleForObjects` :`Start` (`SceneComponent.GetSocketLocation` (`self.Scene`) "None") :`End` (+ (`SceneComponent.GetSocketLocation` (`self.Scene`) "None") (* (`KismetMathLibrary.Normal` (`SceneComponent.GetForwardVector` (`self.Scene`))) 30.0)) :`Radius` 10.0 :`ObjectTypes` (`|MakeArray` "ObjectTypeQuery3" :!type "EObjectTypeQuery Enum") :`DrawDebugType` "ForOneFrame" :`DrawTime` 0.3))
    (if _returnvalue
      (bind (_bblockinghit _binitialoverlap _time _distance _location _impactpoint _normal _impactnormal _physmat _hitactor) (`GameplayStatics.BreakHitResult` _outhit))
      (message `/Game/KEJ/DamageSystem/BPI_Damagable.TakeDamage` _hitactor (make `/Game/KEJ/DamageSystem/S_DamageInfo` 10.0 "NewEnumerator1" "NewEnumerator1"))
      (set `self.leftBtnPressed` false)
      (bind _asbp_darksoul_boss_fight (cast `/Game/KEJ/EJBluePrints/BP_Darksoul_Boss_Fight` _hitactor))
      (`self.PlayAnimMontage` _asbp_darksoul_boss_fight "/Game/KEJ/EJBluePrints/BossMontage.BossMontage" 1.0 (`KismetStringLibrary.Conv_StringToName` (`KismetStringLibrary.Concat_StrStr` "Damage0" (`KismetStringLibrary.Conv_IntToString` (`KismetMathLibrary.RandomIntegerInRange` 1 2))))))))

(fn `CurrentHealth`
  (returns (Health :type "Float (double-precision)"))
  (return (`/Game/KEJ/DamageSystem/BPC_DamageSystem.Health` (`self.BPC_DamageSystem`))))

(fn `GetMaxHealth`
  (returns (MAxHealth :type "Float (double-precision)"))
  (return (`/Game/KEJ/DamageSystem/BPC_DamageSystem.MaxHealth` (`self.BPC_DamageSystem`))))

(fn `TakeDamage`
  (params (DamageInfo :type "/Game/KEJ/DamageSystem/S_DamageInfo Structure"))
  (returns (WasDamaged :type Boolean))
  (bind _wasdamaged (`/Game/KEJ/DamageSystem/BPC_DamageSystem.TakeDamage` (`self.BPC_DamageSystem`) DamageInfo))
  (return _wasdamaged))

(fn `UserConstructionScript`
  (bind _bpc_damagesystem (`self.BPC_DamageSystem`))
  (add `/Game/KEJ/DamageSystem/BPC_DamageSystem.OnDeath` _bpc_damagesystem (`|CreateDelegate` :!event `Death`))
  (add `/Game/KEJ/DamageSystem/BPC_DamageSystem.OnDamageResponse` _bpc_damagesystem (`|CreateDelegate` :!event `DamageResponse`)))
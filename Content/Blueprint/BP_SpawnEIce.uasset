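; BP_SpawnEIce is an actor, apparently an ice attack by its name, that damages the Dark Souls-style boss on contact.
; When HitArea overlaps BP_Darksoul_Boss_Fight, it adds a BPC damage system component to the boss and sends a fixed, typed hit through TakeDamage.
; It then scales up HitArea, adds a particle system component to itself and sets a short lifespan to remove itself.
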(event `self.HitArea.OnComponentBeginOverlap`
  (params (OverlappedComponent :type "PrimitiveComponent Object Reference") (OtherActor :type "Actor Object Reference") (OtherComp :type "PrimitiveComponent Object Reference") (OtherBodyIndex :type Integer) (bFromSweep :type Boolean) (SweepResult :type "HitResult Structure (by ref)"))
  (bind _asbp_darksoul_boss_fight (cast `/Game/KEJ/EJBluePrints/BP_Darksoul_Boss_Fight` OtherActor))
  (`AddComponent|NODE_AddBPC_DamageSystem-0` :`self` _asbp_darksoul_boss_fight)
  (`/Game/KEJ/DamageSystem/BPC_DamageSystem.TakeDamage` (`/Game/KEJ/EJBluePrints/BP_Darksoul_Boss_Fight.BPC_DamageSystem` _asbp_darksoul_boss_fight) (make `/Game/KEJ/DamageSystem/S_DamageInfo` 20.0 "NewEnumerator1"))
  (`SceneComponent.SetWorldScale3D` (`self.HitArea`) (4.0 4.0 4.0))
  (`AddComponent|NODE_AddParticleSystemComponent-1` :`self` (`ActorComponent.GetOwner` (`self.HitArea`)))
  (`self.SetLifeSpan` 7.0))

(fn `UserConstructionScript`)
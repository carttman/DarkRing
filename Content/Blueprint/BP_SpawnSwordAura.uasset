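; BP_SpawnSwordAura is a sword aura actor that damages enemies its HitSword component overlaps.
; The Dark Souls boss receives damage through a BPC damage system component added on each hit, while other enemies lose Hp directly.
; Dogs also get their damaged animation flag set.
; Boss, dog and knight hits add a particle effect to the aura and set a short lifespan for it.
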(event `self.HitSword.OnComponentBeginOverlap`
  (params (OverlappedComponent :type "PrimitiveComponent Object Reference") (OtherActor :type "Actor Object Reference") (OtherComp :type "PrimitiveComponent Object Reference") (OtherBodyIndex :type Integer) (bFromSweep :type Boolean) (SweepResult :type "HitResult Structure (by ref)"))
  (bind _asbp_darksoul_boss_fight (cast `/Game/KEJ/EJBluePrints/BP_Darksoul_Boss_Fight` OtherActor)
    (:`then`
      (`AddComponent|NODE_AddBPC_DamageSystem-0` :`self` _asbp_darksoul_boss_fight)
      (`/Game/KEJ/DamageSystem/BPC_DamageSystem.TakeDamage` (`/Game/KEJ/EJBluePrints/BP_Darksoul_Boss_Fight.BPC_DamageSystem` _asbp_darksoul_boss_fight) (make `/Game/KEJ/DamageSystem/S_DamageInfo` 20.0 "NewEnumerator1")))
    (:`CastFailed`
      (bind _asbp_only_enemy (cast `/Game/Blueprint/Only_BP/BP_OnlyEnemy` OtherActor))
      (set `/Game/Blueprint/Only_BP/BP_OnlyEnemy.Hp` (- (`/Game/Blueprint/Only_BP/BP_OnlyEnemy.Hp` _asbp_only_enemy) 50.0) _asbp_only_enemy)
      (bind _asbp_only_dog_enemy (cast `/Game/Blueprint/Only_BP/BP_OnlyDogEnemy` OtherActor)
        (:`then`
          (set `/Game/Blueprint/Only_BP/ABP_OnlyDogEnemy.isDamaged` true (`/Game/Blueprint/Only_BP/BP_OnlyDogEnemy.anim` _asbp_only_dog_enemy)))
        (:`CastFailed`
          (cast `/Game/Blueprint/Only_BP/BP_OnlyKnightEnemy` OtherActor)))))
  (`AddComponent|NODE_AddParticleSystemComponent-0` :`self` (`ActorComponent.GetOwner` (`self.HitSword`)))
  (`self.SetLifeSpan` 2.0))

(fn `UserConstructionScript`)